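; CountdownGameState is a game state Blueprint that keeps a networked time counter, incrementing it every second on server and clients.
; Every ten counts the authority copies the counter into TimeChecker.
; Its OnRep corrects a drifted local counter and restarts the timer, avoiding per-second replication.
; SetCounter pushes the value to the timer display on player 0's PlayerCharacterBlueprint, caching that character reference.
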(event EventBeginPlay
  (bind _returnvalue (Utilities|Time|SetTimerbyFunctionName 0 "IncreaseCount" 1.0 true))
  (Variables|Default|SetTH_Count _returnvalue))

(event EventTick
  (params (DeltaSeconds :type Float%20%28single-precision%29)))

(fn ConstructionScript)

(fn IncreaseCount
  (bind _result (Math|Integer|IncrementInt (Variables|Default|GetTimeCounter))
    (:%20%20
      (Networking|SwitchHasAuthority
        (:Authority
          (if (== (Math|Integer|%(Integer) _result 10) 9)
            (Variables|Default|SetTimeChecker (Variables|Default|GetTimeCounter))
            (CallFunction|SetCounter)
            (else
              (CallFunction|SetCounter))))
        (:Remote
          (CallFunction|SetCounter))))))

(fn OnRepTimeChecker
  (if (!= (Variables|Default|GetTimeCounter) (Variables|Default|GetTimeChecker))
    (Variables|Default|SetTimeCounter (Variables|Default|GetTimeChecker))
    (Utilities|Time|ClearandInvalidateTimerbyHandle (Variables|Default|GetTH_Count))
    (bind _returnvalue (Utilities|Time|SetTimerbyFunctionName 0 "IncreaseCount" 1.0 true))
    (Variables|Default|SetTH_Count _returnvalue)
    (CallFunction|SetCounter)))

(fn SetCounter
  (bind _returnvalue (Game|GetPlayerController 0))
  (bind _returnvalue_2 (Pawn|GetControlledPawn _returnvalue))
  (Utilities|IsValid (Variables|Default|GetRef%20Char)
    (:Is%20Valid
      _)
    (:Is%20Not%20Valid
      (Utilities|IsValid _returnvalue_2
        (:Is%20Valid
          (bind _asplayer_character_blueprint (Utilities|Casting|CastToPlayerCharacterBlueprint _returnvalue_2))
          (Variables|Default|SetRef%20Char _asplayer_character_blueprint)))))
  (Utilities|IsValid (Variables|/Game/Blueprints/PlayerCharacterBlueprint.PlayerCharacterBlueprint_C|GetRef%20Timer%20Display (Variables|Default|GetRef%20Char))
    (:Is%20Valid
      (Default|UpdateTime (Variables|/Game/Blueprints/PlayerCharacterBlueprint.PlayerCharacterBlueprint_C|GetRef%20Timer%20Display (Variables|Default|GetRef%20Char)) (Variables|Default|GetTimeCounter)))))